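; Survival game mode that assigns each player their own spawn point from the BP_SurvivalPlayerStart actors in the level.
; FindPlayerStart fills the PlayerStarts list through FindStarts when it is empty, then returns the first unused start and marks it used.
; A random-pick variant that rerolls until it hits a free start is present but never runs.
; No fallback is wired for when every start is used.
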(event Custom|Find%20Starts
  (bind _outactors (Actor|GetAllActorsOfClass "/Game/Blueprints/BP_SurvivalPlayerStart.BP_SurvivalPlayerStart_C"))
  (Variables|Default|SetPlayerStarts _outactors))

(fn ConstructionScript)

(fn FindPlayerStart
  (params (Player :type Controller%20Object%20Reference) (IncomingName :type String))
  (if (<= (Utilities|Array|Length (Variables|Default|GetPlayerStarts)) 0)
    (CallFunction|FindStarts))
  (for _array_element (Variables|Default|GetPlayerStarts)
    (if (not (Variables|/Game/Blueprints/BP_SurvivalPlayerStart.BP_SurvivalPlayerStart_C|GetUsed _array_element))
      (Default|MarkUsed _array_element)
      (return _array_element))))