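; Survival character Blueprint that handles hit feedback and sets up a scene capture of itself.
; PointDamage calls PlayHitFX, which plays a random hit-react montage and spawns blood at the impact, oriented to the surface normal, for point damage.
; The construction script adds the character to its SceneCaptureComponent2D's show-only actors.
; An unconnected, authority-only branch would grant a starting M14 and ammo, but never runs.
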(event Custom|Play%20Hit%20FX
  (params (Damage :type Float%20%28single-precision%29) (DamageType :type Damage%20Type%20Object%20Reference) (Hit :type Hit%20Result%20Structure) (IsPointDamage :type Boolean))
  (bind (_bblockinghit _binitialoverlap _time _distance _location _impactpoint _normal _impactnormal) (Collision|BreakHitResult Hit))
  (bind _hitreactanimations (Variables|FX|GetHitReactAnimations))
  (Animation|PlayAnimMontage (Utilities|Array|Get(acopy) _hitreactanimations (Math|Random|RandomIntegerinRange 0 (- (Utilities|Array|Length _hitreactanimations) 1))) 1.0 "None")
  (if IsPointDamage
    (Effects|SpawnEmitteratLocation "/Game/Particles/P_Blood.P_Blood" _location (Math|Conversions|RotationFromXVector _impactnormal))))

(event EventBeginPlay)

(event Game|Damage|EventPointDamage
  (params (Damage :type Float%20%28single-precision%29) (DamageType :type Damage%20Type%20Object%20Reference) (HitLocation :type Vector :default "0, 0, 0") (HitNormal :type Vector :default "0, 0, 0") (HitComponent :type Primitive%20Component%20Object%20Reference) (BoneName :type Name :default "None") (ShotFromDirection :type Vector :default "0, 0, 0") (InstigatedBy :type Controller%20Object%20Reference) (DamageCauser :type Actor%20Object%20Reference) (HitInfo :type Hit%20Result%20Structure%20%28by%20ref%29))
  (CallFunction|PlayHitFX Damage DamageType HitInfo true))

(fn ConstructionScript
  (Utilities|Array|AddUnique (Variables|/Script/Engine.SceneCaptureComponent|GetShowOnlyActors (Variables|Default|GetSceneCaptureComponent2D)) self))